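; Scene camera actor for the visual novel framework that frames characters, copying the player camera's post-process settings and applying per-scene or closeup blur.
; Moving to it can play a timeline slide whose side is computed from the previous camera's angle, notifying viewed characters.
; Jump, zoom and random-angle events offset the camera from its origin, and Tick interpolates handheld shake.
; It also shows CG images through widget or sprite fills.
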(event Custom|JumpCam
  (params (Zoom? :type Boolean) (Horizontal? :type Boolean) (JumpAmount :type Float%20%28single-precision%29) (CharHorizontal :type Float%20%28single-precision%29))
  (bind _rootscenecomponent (Variables|Default|GetRootSceneComponent))
  (bind _originpoint (Variables|Default|GetoriginPoint))
  (bind _originpoint_2 (Variables|Default|GetoriginPoint))
  (if Zoom?
    ;[1 1 1] Zoom
    (if (not (Variables|Default|GetZoomedIn?)) ; only zoom if not already zoomed
      (if (Variables|Default|GetCloseupCam?)
        (Variables|Default|SetcurrentAngleLoc (+ (+ (+ (Variables|Default|GetcurrentAngleLoc) (* (Math|Vector|GetForwardVector _rootscenecomponent) JumpAmount)) (* (Math|Vector|GetUpVector _rootscenecomponent) (* JumpAmount 0.35))) (* (Math|Vector|GetRightVector _rootscenecomponent) (* CharHorizontal 0.2)))) ; re-center closeup cameras
        (else
          (Variables|Default|SetcurrentAngleLoc (+ (+ (Variables|Default|GetcurrentAngleLoc) (* (Math|Vector|GetForwardVector _rootscenecomponent) JumpAmount)) (* (Math|Vector|GetUpVector _rootscenecomponent) (* JumpAmount 0.35))))))
      (Transformation|SetWorldLocationAndRotation _rootscenecomponent (Variables|Default|GetcurrentAngleLoc) (.rotation (Variables|Default|GetoriginPoint)) false false)
      (Variables|Default|SetZoomedIn? true)
      (if (Variables|Default|Getshaking) :!label _label
        ;[1 1 1] adjust if shaking
        (Variables|Default|SetShakeVector (Variables|Default|GetcurrentAngleLoc))))
    (elif Horizontal?
      (bind _output_get (Variables|Default|SetcurrentAngleLoc (+ (.location _originpoint) (* (Math|Vector|GetRightVector _rootscenecomponent) JumpAmount))))
      (Transformation|SetWorldLocationAndRotation _rootscenecomponent _output_get (.rotation _originpoint) false false)
      (goto _label)
      (else
        (bind _output_get_2 (Variables|Default|SetcurrentAngleLoc (+ (.location _originpoint_2) (* (Math|Vector|GetUpVector _rootscenecomponent) JumpAmount))))
        (Transformation|SetWorldLocationAndRotation _rootscenecomponent _output_get_2 (.rotation _originpoint_2) false false)
        (goto _label)))))

(event Custom|RegCam
  (params (CharPushedBack? :type Boolean) (CharActor :type Parent%20Actor%20Object%20Reference))
  (Variables|Default|SetZoomedIn? false)
  (Variables|Default|SetRandAngles? false)
  (CallFunction|JumpCam false true 0.0 0.0)
  (Default|CamReg CharActor))

(event Custom|RandJump
  (params (CharPushedBack? :type Boolean))
  (if (Variables|Default|GetRandAngles?)
    _
    (else
      (Variables|Default|SetCharacterPushedBack? CharPushedBack?)
      (Variables|Default|SetRandAngles? true)))
  (switch int (Math|Random|RandomIntegerinRange 0 6)
    (:0
      (CallFunction|RegRandom :!label _label))
    (:1
      (CallFunction|JumpLeft (Variables|Default|GetCharacterPushedBack?)))
    (:2
      (CallFunction|JumpRight (Variables|Default|GetCharacterPushedBack?)))
    (:3
      (CallFunction|JumpUp (Variables|Default|GetCharacterPushedBack?)))
    (:4
      (CallFunction|Zoomin (Variables|Default|GetCharacterPushedBack?) :!label _label_2))
    (:5
      (goto _label_2))
    (:6
      (goto _label)))
  (Utilities|FlowControl|Delay (Math|Conversions|ToFloat(Integer) (Math|Random|RandomIntegerinRange 2 4)))
  (if (Variables|Default|GetRandAngles?)
    (CallFunction|RandJump (Variables|Default|GetCharacterPushedBack?))))

(event Custom|InitVariables
  ;[0.2633 1 0.5891] Begin Setup
  (bind _output_get (Variables|Default|SetoriginPoint (Transformation|GetWorldTransform (Variables|Default|GetSceneComponent))))
  (Variables|Default|SetcharSquareOriginPoint (Transformation|GetWorldTransform (Variables|Default|GetCharRotationSquare)))
  (Variables|Default|SetcurrentAngleLoc (.location _output_get))
  (Variables|Default|SetShakeVector (.location _output_get))
  (Variables|Default|SetRootSceneComponent (VehicleSound|GetRootComponent))
  (Variables|Default|SetLocalCamera (Variables|CameraActor|GetCameraComponent))
  (Rendering|SetVisibility (Variables|Default|GetSprite_ImageFill) false false))

(event Custom|ImageFill
  (params (WidgetMode? :type Boolean) (newCG :type String))
  (bind _widget_imagefill (Variables|Default|GetWidget_ImageFill))
  (bind _sprite_imagefill (Variables|Default|GetSprite_ImageFill))
  ;[0.609 1 0.6856] CG control
  (bind _aswd_cg (Utilities|Casting|CastToWD_CG (UserInterface|GetUserWidgetObject _widget_imagefill)))
  (if WidgetMode?
    (Default|SetCGInit _aswd_cg newCG)
    (Rendering|SetVisibility _widget_imagefill true false)
    (else
      (bind (_sprite _texture2d _sprite_) (Default|UnlockPersistentData _aswd_cg newCG "/Game/VN_Framework/Gallery/GalleryListDT.GalleryListDT"))
      (if _sprite_
        (Rendering|Components|Sprite|SetSprite _sprite_imagefill _sprite)
        (Rendering|SetVisibility _sprite_imagefill true false)))))

(event Custom|ShowCGWidget
  ;[0.609 1 0.6856] CG control
  (Rendering|SetVisibility (Variables|Default|GetWidget_ImageFill) true false)
  (bind _asglobal_bp (Utilities|Casting|CastToGlobal_BP (Game|GetGameInstance)))
  (Default|In-SceneCamBlur _asglobal_bp 1 self))

(event Custom|RegRandom
  (Variables|Default|SetZoomedIn? false)
  (CallFunction|JumpCam false true 0.0 0.0))

(event Custom|HideCGWidget
  (bind _widget_imagefill (Variables|Default|GetWidget_ImageFill))
  (bind _scenetemplate (Variables|Default|GetSceneTemplate))
  ;[0.609 1 0.6856] CG control
  (if (Variables|/Script/Engine.SceneComponent|GetbVisible _widget_imagefill)
    (Rendering|SetVisibility _widget_imagefill false false)
    (if (Variables|Default|GetCloseupCam?)
      (CallFunction|CloseupBlur)
      (else
        (Utilities|IsValid _scenetemplate
          (:Is%20Valid
            (Default|In-SceneCamBlur (Variables|/Game/VN_Framework/Blueprints/SceneTemplate_BP.SceneTemplate_BP_C|GetGlobal_BP _scenetemplate) (.bluramount (Variables|/Game/VN_Framework/Blueprints/SceneTemplate_BP.SceneTemplate_BP_C|GetSceneData _scenetemplate)) self)))))))

(event Custom|SlideGo
  (bind _rootscenecomponent (Variables|Default|GetRootSceneComponent))
  (bind _slidemultiplier (Variables|Slide|GetSlideMultiplier))
  (bind _currentangleloc (Variables|Default|GetcurrentAngleLoc))
  (bind _originpoint (Variables|Default|GetoriginPoint))
  (bind _returnvalue (Math|Vector|GetRightVector _rootscenecomponent))
  (bind _returnvalue_2 (* _returnvalue _slidemultiplier))
  (bind _returnvalue_3 (+ _currentangleloc _returnvalue_2))
  ;[1 1 1] Slide Camera
  (if (Variables|Default|GetInitialized?)
    (Utilities|Struct|SetmembersinPostProcessSettings (Variables|/Script/Engine.CameraComponent|GetPostProcessSettings (Variables|CameraActor|GetCameraComponent)) 1.0 1.0)
    (Transformation|SetWorldLocationAndRotation (Variables|Default|GetLocalCamera) _returnvalue_3 (.rotation (Variables|Default|GetoriginPoint)) false false)
    (bind _alpha (Timeline|Timeline_0 PlayFromStart)
      (:Update
        (Transformation|SetWorldLocationAndRotation (Variables|Default|GetLocalCamera) (.location (Math|Transform|Lerp(Transform) (Math|Transform|MakeTransform _returnvalue_3 (Transformation|GetWorldRotation _rootscenecomponent) "1,1,1") (Math|Transform|MakeTransform (Variables|Default|GetcurrentAngleLoc) (.rotation _originpoint) (.scale _originpoint)) _alpha)) (.rotation (Math|Transform|Lerp(Transform) (Math|Transform|MakeTransform _returnvalue_3 (Transformation|GetWorldRotation _rootscenecomponent) "1,1,1") (Math|Transform|MakeTransform (Variables|Default|GetcurrentAngleLoc) (.rotation _originpoint) (.scale _originpoint)) _alpha)) false false))
      (:Finished
        (bind _asglobal_bp (Utilities|Casting|CastToGlobal_BP (Game|GetGameInstance)))
        (bind _asvn_first_person_character (Utilities|Casting|CastToVN_FirstPersonCharacter (Variables|/Game/VN_Framework/Blueprints/Global_BP.Global_BP_C|GetPlayerActor _asglobal_bp)))
        (Utilities|Struct|SetmembersinPostProcessSettings (Variables|/Script/Engine.CameraComponent|GetPostProcessSettings (Variables|CameraActor|GetCameraComponent)) (.DepthOfFieldFocalDistance (Utilities|Struct|BreakPostProcessSettings (Variables|/Script/Engine.CameraComponent|GetPostProcessSettings (Variables|/Game/VN_Framework/Blueprints/VN_FirstPersonCharacter.VN_FirstPersonCharacter_C|GetFirstPersonCamera _asvn_first_person_character)))) (.DepthOfFieldFocalRegion (Utilities|Struct|BreakPostProcessSettings (Variables|/Script/Engine.CameraComponent|GetPostProcessSettings (Variables|/Game/VN_Framework/Blueprints/VN_FirstPersonCharacter.VN_FirstPersonCharacter_C|GetFirstPersonCamera _asvn_first_person_character)))) (.DepthOfFieldScale (Utilities|Struct|BreakPostProcessSettings (Variables|/Script/Engine.CameraComponent|GetPostProcessSettings (Variables|/Game/VN_Framework/Blueprints/VN_FirstPersonCharacter.VN_FirstPersonCharacter_C|GetFirstPersonCamera _asvn_first_person_character)))) (.MotionBlurAmount (Utilities|Struct|BreakPostProcessSettings (Variables|/Script/Engine.CameraComponent|GetPostProcessSettings (Variables|/Game/VN_Framework/Blueprints/VN_FirstPersonCharacter.VN_FirstPersonCharacter_C|GetFirstPersonCamera _asvn_first_person_character)))) (.MotionBlurMax (Utilities|Struct|BreakPostProcessSettings (Variables|/Script/Engine.CameraComponent|GetPostProcessSettings (Variables|/Game/VN_Framework/Blueprints/VN_FirstPersonCharacter.VN_FirstPersonCharacter_C|GetFirstPersonCamera _asvn_first_person_character)))))))
    (else
      (Utilities|FlowControl|Delay (* (Utilities|Time|GetWorldDeltaSeconds) 3.0))
      (CallFunction|SlideGo))))

(event Custom|CloseupBlur
  ;[1 1 1] Closeup Begin
  (Utilities|Struct|SetmembersinPostProcessSettings (Variables|/Script/Engine.CameraComponent|GetPostProcessSettings (Variables|CameraActor|GetCameraComponent)) 2e+01))

(event Custom|SceneCamSettings
  (params (SceneTemplate :type Scene%20Template%20BP%20Object%20Reference))
  ;[0.2633 1 0.5891] Begin Setup
  (Utilities|IsValid SceneTemplate
    (:Is%20Valid
      (Default|In-SceneCamBlur (Variables|/Game/VN_Framework/Blueprints/SceneTemplate_BP.SceneTemplate_BP_C|GetGlobal_BP SceneTemplate) (.bluramount (Variables|/Game/VN_Framework/Blueprints/SceneTemplate_BP.SceneTemplate_BP_C|GetSceneData SceneTemplate)) self))))

(event Custom|Screenshot
  (bind _returnvalue (AddComponent|AddSceneCaptureComponent2D false (Math|Transform|MakeTransform "0, 0, 0")))
  (Variables|Default|SetSceneCapture _returnvalue)
  (Variables|/Script/Engine.SceneCaptureComponent2D|SetTextureTarget (Variables|Default|GetSceneCapture) 0)
  (Rendering|SceneCapture|CaptureScene (Variables|Default|GetSceneCapture) :!class /Script/Engine.SceneCaptureComponent2D)
  (Components|DestroyComponent (Variables|Default|GetSceneCapture)))

(event Custom|InitiateCloseup
  (params (CharXValue :type Float%20%28single-precision%29) (PlayerChar :type VN%20First%20Person%20Character%20Object%20Reference) (SceneTemplate :type Scene%20Template%20BP%20Object%20Reference))
  ;[1 1 1] Closeup Begin
  (if (not (Variables|Default|GetCloseupCam?))
    (Utilities|FlowControl|Sequence
      (:then_0
        (if (not (Variables|Default|GetInitialized?))
          (CallFunction|MidSceneNewCam PlayerChar SceneTemplate)))
      (:then_1
        (Variables|Default|SetCloseupCam? true)
        (Utilities|Struct|SetmembersinPostProcessSettings (Variables|/Script/Engine.CameraComponent|GetPostProcessSettings (Variables|CameraActor|GetCameraComponent)) 2e+01)))))

(event Custom|JumpUp
  (params (CharPushedBack? :type Boolean))
  (bind _finaladjustment (CallFunction|AdjustCamFloat CharPushedBack? 3e+01))
  (CallFunction|JumpCam false false _finaladjustment 0.0))

(event Custom|SlideInit
  (params (LetCamAutoCalculateSlide? :type Boolean) (SlideMultiplier :type Float%20%28single-precision%29) (PreviousViewTarget :type Actor%20Object%20Reference))
  (bind _charactersviewed (Variables|Default|GetCharactersViewed))
  ;[1 1 1] Initiate Slide
  (if (Variables|Slide|GetEnableSlide?)
    (if LetCamAutoCalculateSlide?
      (if (Variables|Default|GetCloseupCam?)
        (if (Variables|Default|GetSkippedSlide)
          (bind _asmain_camera (Utilities|Casting|CastToMainCamera PreviousViewTarget)) ; only slide for closeups from another closeup
          (if (Variables|MainCamera_C|GetCloseupCam? _asmain_camera)
            (Variables|Slide|SetSlideMultiplier 4e+01)
            (CallFunction|CalculateSlide PreviousViewTarget :!label _label)
            (for _array_element _charactersviewed
              (Utilities|IsValid _array_element
                (:Is%20Valid
                  (if (not (Variables|/Game/VN_Framework/Blueprints/ParentActor.ParentActor_C|GetPendingDestruct _array_element))
                    (Default|CameraSliding _array_element (Variables|Slide|GetSlideMultiplier)) ; tell character about slide
                    (else
                      (Utilities|Array|RemoveItem _charactersviewed _array_element :!label _label_2))))
                (:Is%20Not%20Valid
                  (goto _label_2)))))
          (else
            (Variables|Default|SetSkippedSlide true) ; skip slide the very first time
          ))
        (else
          (bind _asmain_camera_2 (Utilities|Casting|CastToMainCamera PreviousViewTarget)
            (:then
              (if (not (Variables|MainCamera_C|GetCloseupCam? _asmain_camera_2))
                (Variables|Slide|SetSlideMultiplier 7e+01 :!label _label_3)
                (goto _label)))
            (:CastFailed
              (goto _label_3)))))
      (else
        (Variables|Slide|SetSlideMultiplier SlideMultiplier)))))

(event Custom|ResetLocation
  (bind _output_get (Variables|Default|SetoriginPoint (Transformation|GetWorldTransform (Variables|Default|GetSceneComponent))))
  (Variables|Default|SetcharSquareOriginPoint (Transformation|GetWorldTransform (Variables|Default|GetCharRotationSquare)))
  (Variables|Default|SetcurrentAngleLoc (.location _output_get))
  (Variables|Default|SetShakeVector (.location _output_get)))

(event Custom|JumpLeft
  (params (CharPushedBack? :type Boolean))
  (bind _finaladjustment (CallFunction|AdjustCamFloat false -1e+02))
  (CallFunction|JumpCam false true _finaladjustment 0.0))

(event Custom|JumpRight
  (params (CharPushedBack? :type Boolean))
  (bind _finaladjustment (CallFunction|AdjustCamFloat CharPushedBack? 1e+02))
  (CallFunction|JumpCam false true _finaladjustment 0.0))

(event Custom|PlayerCamSettings
  (params (PlayerChar :type Object%20Object%20Reference))
  (bind _cameracomponent (Variables|CameraActor|GetCameraComponent))
  ;[0.2633 1 0.5891] Begin Setup
  (Utilities|IsValid _cameracomponent
    (:Is%20Valid
      (bind _asvn_first_person_character (Utilities|Casting|CastToVN_FirstPersonCharacter PlayerChar)
        (:then
          (Variables|/Script/Engine.CameraComponent|SetPostProcessSettings _cameracomponent (Variables|/Script/Engine.CameraComponent|GetPostProcessSettings (Variables|/Game/VN_Framework/Blueprints/VN_FirstPersonCharacter.VN_FirstPersonCharacter_C|GetFirstPersonCamera _asvn_first_person_character))))
        (:CastFailed
          (Development|PrintString "camera not valid" :!label _label))))
    (:Is%20Not%20Valid
      (goto _label))))

(event Custom|MidSceneNewCam
  (params (PlayerChar :type VN%20First%20Person%20Character%20Object%20Reference) (SceneTemplateBP :type Scene%20Template%20BP%20Object%20Reference))
  ;[0.2633 1 0.5891] Begin Setup
  (CallFunction|InitVariables)
  (Variables|Default|SetSceneTemplate SceneTemplateBP)
  (CallFunction|PlayerCamSettings PlayerChar)
  (Utilities|FlowControl|Sequence
    (:then_0
      (Variables|Default|SetInitialized? true))
    (:then_1
      (CallFunction|SceneCamSettings SceneTemplateBP))))

(event Custom|ZoomIn
  (params (CharPushedBack? :type Boolean) (CharActor :type Parent%20Actor%20Object%20Reference))
  (bind _finaladjustment (CallFunction|AdjustCamFloat CharPushedBack? (Transformation|GetDistanceTo CharActor)))
  (CallFunction|JumpCam true false _finaladjustment (.x (Variables|/Game/VN_Framework/Blueprints/ParentActor.ParentActor_C|GetCharVectorConstant CharActor)))
  (Default|CamZoom CharActor))

(event EventBeginPlay
  ;[0.2633 1 0.5891] Begin Setup
  (CallFunction|InitVariables))

(event Collision|EventActorBeginOverlap
  (params (OtherActor :type Actor%20Object%20Reference)))

(event EventOnEndViewTarget
  (params (PC :type Player%20Controller%20Object%20Reference)))

(event EventCGEnd
  (params (Instant? :type Boolean) (CGWidget :type WD%20CG%20Object%20Reference))
  ;[0.609 1 0.6856] CG control
  (CallFunction|HideCGWidget))

(event EventCamUpdate
  (params (Player :type VN%20First%20Person%20Character%20Object%20Reference))
  ;[0.2633 1 0.5891] Begin Setup
  (if (Variables|Default|GetInitialized?)
    _
    (else
      (CallFunction|InitVariables)))
  (CallFunction|PlayerCamSettings Player)
  (Variables|Default|SetInitialized? true)
  (bind _asglobal_bp (Utilities|Casting|CastToGlobal_BP (Game|GetGameInstance)))
  (if (Variables|/Game/VN_Framework/Blueprints/Global_BP.Global_BP_C|GetScenePlaying? _asglobal_bp)
    (if (Variables|Default|GetCloseupCam?)
      (CallFunction|CloseupBlur)
      (else
        (bind _outactors (Actor|GetAllActorsOfClass "/Game/VN_Framework/Blueprints/SceneTemplate_BP.SceneTemplate_BP_C"))
        (Utilities|IsValid (Utilities|Array|Get(acopy) _outactors)
          (:Is%20Valid
            (CallFunction|SceneCamSettings (Utilities|Array|Get(acopy) _outactors))))))))

(event EventOnBecomeViewTarget
  (params (PC :type Player%20Controller%20Object%20Reference)))

(event EventShakyStepEvent
  (params (RandomX :type Float%20%28single-precision%29) (RandomY :type Float%20%28single-precision%29) (RandomScale :type Float%20%28single-precision%29))
  (bind _cameracomponent (Variables|CameraActor|GetCameraComponent))
  (bind _randomstream (Variables|Default|GetRandomStream))
  ;[1 0.9027 0.4983] Shake handheld camera effects
  (Variables|Default|SetShakeVector (+ (* (Math|Vector|GetRightVector _cameracomponent) RandomX) (+ (Variables|Default|GetcurrentAngleLoc) (* (Math|Vector|GetUpVector _cameracomponent) RandomY))))
  (Math|Random|SetRandomStreamSeed _randomstream (.Millisecond (Math|DateTime|BreakDateTime (Math|DateTime|Now))))
  (Class|KismetMathLibrary|ResetRandomStream _randomstream))

(event EventShakeEnd
  ;[1 0.9027 0.4983] Shake handheld camera effects
  (Variables|Default|Setshaking false))

(event EventTick
  (params (DeltaSeconds :type Float%20%28single-precision%29))
  (bind _cameracomponent (Variables|CameraActor|GetCameraComponent))
  ;[1 0 0.04978] Event tick
  (if (Variables|Default|Getshaking)
    (Transformation|SetWorldLocation _cameracomponent (Math|Interpolation|VInterpTo (Transformation|GetWorldLocation _cameracomponent) (Variables|Default|GetShakeVector) DeltaSeconds (Variables|Default|GetTerpTime)) false false)))

(event EventShakeInitiate
  ;[1 0.9027 0.4983] Shake handheld camera effects
  (Variables|Default|Setshaking true))

(event EventLevelReady
  (params (Player :type VN%20First%20Person%20Character%20Object%20Reference))
  ;[0.2633 1 0.5891] Begin Setup
  (CallFunction|PlayerCamSettings Player)
  (Variables|Default|SetInitialized? true))

(event EventSceneInitStart
  (params (sceneTemplate :type Scene%20Template%20BP%20Object%20Reference))
  ;[0.2633 1 0.5891] Begin Setup
  (CallFunction|SceneCamSettings sceneTemplate))

(event EventCGstart
  (params (CGNickname :type String) (InitCam :type Main%20Camera%20Object%20Reference) (ZoomPivot :type Vector :default "0, 0, 0") (CGCreated :type WD%20CG%20Object%20Reference))
  ;[0.609 1 0.6856] CG control
  (UserInterface|SetWidget (Variables|Default|GetWidget_ImageFill) CGCreated)
  (if (== InitCam self)
    (CallFunction|ShowCGWidget)))

(event EventCGCamSwitch
  (params (NewCam :type Main%20Camera%20Object%20Reference) (CG_Widget :type WD%20CG%20Object%20Reference))
  ;[0.609 1 0.6856] CG control
  (if (== NewCam self)
    (CallFunction|ShowCGWidget)
    (else
      (CallFunction|HideCGWidget))))

(fn ConstructionScript)

(fn CalculateClockwiseRotation
  (params (PreviousView :type Actor%20Object%20Reference))
  (bind _returnvalue (Transformation|GetActorRotation PreviousView))
  (bind _returnvalue_2 (Transformation|GetActorLocation))
  (bind _returnvalue_3 (Transformation|GetActorLocation PreviousView))
  (bind _returnvalue_4 (Math|Vector|GetUnitDirection(Vector) _returnvalue_3 _returnvalue_2))
  (bind _returnvalue_5 (Math|Vector|GetRightVector _returnvalue))
  (if (< (Class|KismetMathLibrary|DegAcos (/ (Math|Vector|DotProduct _returnvalue_5 _returnvalue_4) (* (Math|Vector|VectorLength _returnvalue_5) (Math|Vector|VectorLength _returnvalue_4)))) 1e+02)
    (Variables|Slide|SetSlideMultiplier -5e+01)
    (else
      (Variables|Slide|SetSlideMultiplier 5e+01)))
  (CallFunction|SlideGo))

(fn CalculateSlide
  (params (previous%20cam :type Actor%20Object%20Reference))
  (bind _returnvalue (Transformation|GetActorRotation previous%20cam))
  (bind _returnvalue_2 (Transformation|GetActorLocation))
  (bind _returnvalue_3 (Transformation|GetActorLocation previous%20cam))
  (bind _returnvalue_4 (Math|Vector|GetUnitDirection(Vector) _returnvalue_3 _returnvalue_2))
  (bind _returnvalue_5 (Math|Vector|GetRightVector _returnvalue))
  (if (< (Class|KismetMathLibrary|DegAcos (/ (Math|Vector|DotProduct _returnvalue_5 _returnvalue_4) (* (Math|Vector|VectorLength _returnvalue_5) (Math|Vector|VectorLength _returnvalue_4)))) (Variables|Slide|GetSlideAngle))
    (Variables|Slide|SetSlideMultiplier (* -1 (Math|Float|Absolute(Float) (Variables|Slide|GetSlideMultiplier))))
    (else
      (Variables|Slide|SetSlideMultiplier (Math|Float|Absolute(Float) (Variables|Slide|GetSlideMultiplier)))))
  (CallFunction|SlideGo))

(fn AdjustCamFloat
  (params (PushedBack? :type Boolean) (JumpFloat :type Float%20%28single-precision%29))
  (return (* JumpFloat 0.13)))

(fn CheckWidget
  (params (Show? :type Boolean))
  (bind _scenetemplate (Variables|Default|GetSceneTemplate))
  (if (Variables|Default|GetInitialized?)
    (Utilities|IsValid _scenetemplate
      (:Is%20Valid
        (Utilities|IsValid (Variables|/Game/VN_Framework/Blueprints/SceneTemplate_BP.SceneTemplate_BP_C|GetCGwidget _scenetemplate)
          (:Is%20Valid
            (if Show?
              (CallFunction|ShowCGWidget)
              (else
                (CallFunction|HideCGWidget)))))))))

(fn GetSceneCapture
  (bind _scenecapture (Variables|Default|GetSceneCapture))
  (Rendering|SceneCapture|CaptureScene _scenecapture :!class /Script/Engine.SceneCaptureComponent2D)
  (return _scenecapture))

(fn SceneEnd
  (params (SceneTemplateBP :type Scene%20Template%20BP%20Object%20Reference) (next_scene :type String) (next_subLevel :type String) (next%20map%20Level :type String))
  (return false))

(fn SceneModeStart
  (params (SceneTouchClickSource :type Touch%20Click%20Actor%20BP%20Object%20Reference) (SceneTemplateBP :type Scene%20Template%20BP%20Object%20Reference))
  (Variables|Default|SetSceneTemplate SceneTemplateBP)
  (if (not (Variables|Default|GetInitialized?))
    (bind _asglobal_bp (Utilities|Casting|CastToGlobal_BP (Game|GetGameInstance)))
    (bind _asvn_first_person_character (Utilities|Casting|CastToVN_FirstPersonCharacter (Variables|/Game/VN_Framework/Blueprints/Global_BP.Global_BP_C|GetPlayerActor _asglobal_bp)))
    (CallFunction|MidSceneNewCam _asvn_first_person_character SceneTemplateBP)))